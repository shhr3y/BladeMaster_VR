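; BP_Enemy is an enemy actor that the player destroys with a saber to earn points in a VR game.
; On BeginPlay it caches the player's VRPawn.
; When EnemyObject overlaps a BP_Saber, it adds score through that pawn, spawns an NS_Explosion effect offset from the hit component, and destroys itself.
; A world camera shake node is present but unconnected, so it never runs.
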(event `self.ReceiveBeginPlay`
  (bind _asvrpawn (cast `/Game/VRTemplate/Blueprints/VRPawn` (`GameplayStatics.GetPlayerPawn` 0)))
  (set `self.User Ref` _asvrpawn))

(event `self.EnemyObject.OnComponentBeginOverlap`
  (params (OverlappedComponent :type "PrimitiveComponent Object Reference") (OtherActor :type "Actor Object Reference") (OtherComp :type "PrimitiveComponent Object Reference") (OtherBodyIndex :type Integer) (bFromSweep :type Boolean) (SweepResult :type "HitResult Structure (by ref)"))
  (bind (_x _y _z) (`KismetMathLibrary.BreakVector3f` (`SceneComponent.K2_GetComponentLocation` OverlappedComponent)))
  (cast `/Game/VRTemplate/Blueprints/BP_Saber` OtherActor)
  (`/Game/VRTemplate/Blueprints/VRPawn.Update User Score` (`self.User Ref`) 5)
  (`NiagaraFunctionLibrary.SpawnSystemAtLocation` "/Game/InfiniteMatrix/VFX/NS_Explosion.NS_Explosion" (`KismetMathLibrary.MakeVector` _x (- _y 300.0) (+ _z 50.0)))
  (`self.K2_DestroyActor`))

(fn `UserConstructionScript`)