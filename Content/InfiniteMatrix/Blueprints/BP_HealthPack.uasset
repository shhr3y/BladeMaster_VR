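; BP_HealthPack is a health pickup for the VR player that slowly spins around its vertical axis.
; It caches the player's VRPawn on BeginPlay.
; When a BP_Saber overlaps its sphere, it calls UpdateUserHealth on that pawn to add health, then destroys itself, so collection happens by saber contact rather than body contact.
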(event `self.ReceiveBeginPlay`
  (bind _asvrpawn (cast `/Game/VRTemplate/Blueprints/VRPawn` (`GameplayStatics.GetPlayerPawn` 0)))
  (set `self.User Ref` _asvrpawn))

(event `self.ReceiveTick`
  (params (DeltaSeconds :type "Float (single-precision)"))
  (`SceneComponent.K2_AddLocalRotation` (`self.HealthPack`) (`KismetMathLibrary.MakeRotator` 0.0 0.0 (* DeltaSeconds 60.0)) false false))

(event `self.Sphere.OnComponentBeginOverlap`
  (params (OverlappedComponent :type "PrimitiveComponent Object Reference") (OtherActor :type "Actor Object Reference") (OtherComp :type "PrimitiveComponent Object Reference") (OtherBodyIndex :type Integer) (bFromSweep :type Boolean) (SweepResult :type "HitResult Structure (by ref)"))
  (cast `/Game/VRTemplate/Blueprints/BP_Saber` OtherActor)
  (`/Game/VRTemplate/Blueprints/VRPawn.UpdateUserHealth` (`self.User Ref`) 10.0)
  (`self.K2_DestroyActor`))

(fn `UserConstructionScript`)