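; Spawner actor that builds a chain of BP_Tunnel segments and populates them with enemies and health packs.
; On BeginPlay it destroys existing tunnels, then spawns an initial run from the player pawn, chaining each at the newest segment's SpawnPoint.
; Each tunnel receives a reference back to the spawner.
; Each spawn adds an enemy and occasionally a health pack at random offsets, both with limited lifespans.
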(event `self.ReceiveBeginPlay`
  (`self.SpawnInitialTunnels`))

(fn `AddRandomEnemy`
  (params (Location :type "Vector Structure"))
  (if true
    (bind _returnvalue (`|SpawnActorFromClass` "/Game/InfiniteMatrix/Blueprints/BP_Enemy.BP_Enemy_C" (`KismetMathLibrary.MakeTransform` (`KismetMathLibrary.MakeVector` (+ (.x Location) (`KismetMathLibrary.RandomFloatInRange` 400.0 1850.0)) (+ (.y Location) (`KismetMathLibrary.RandomFloatInRange` -300.0 300.0)) (+ (.z Location) (`KismetMathLibrary.RandomFloatInRange` -400.0 250.0)))) "Undefined" "OverrideRootScale" null null))
    (`self.SetLifeSpan` _returnvalue 20.0)))

(fn `AddRandomHealthPack`
  (params (InVec :type "Vector Structure"))
  (if (> (`KismetMathLibrary.RandomIntegerInRange` 0 9) 7)
    (bind _returnvalue (`|SpawnActorFromClass` "/Game/InfiniteMatrix/Blueprints/BP_HealthPack.BP_HealthPack_C" (`KismetMathLibrary.MakeTransform` (`KismetMathLibrary.MakeVector` (+ (.x InVec) (`KismetMathLibrary.RandomFloatInRange` 400.0 1850.0)) (+ (.y InVec) (`KismetMathLibrary.RandomFloatInRange` -300.0 300.0)) (+ (.z InVec) (`KismetMathLibrary.RandomFloatInRange` -400.0 250.0)))) "Undefined" "OverrideRootScale" null null))
    (`self.SetLifeSpan` _returnvalue 20.0)))

(fn `Spawn Tunnel at Spawn Point`
  (`self.SpawnTunnel` (`SceneComponent.K2_GetComponentLocation` (`/Game/InfiniteMatrix/Blueprints/BP_Tunnel.SpawnPoint` (`self.Newest Tunnel`)))))

(fn `SpawnInitialTunnels`
  (`|ExecutionSequence`
    (:`then_0`
      (bind _outactors (`GameplayStatics.GetAllActorsOfClass` "/Game/InfiniteMatrix/Blueprints/BP_Tunnel.BP_Tunnel_C"))
      (for _array_element _outactors
        (`self.K2_DestroyActor` _array_element)))
    (:`then_1`
      (for _ (range 7)
        (`/Engine/EditorBlueprintResources/StandardMacros.IsValid` (`self.Newest Tunnel`)
          (:`Is Valid`
            (`self.Spawn Tunnel at Spawn Point`))
          (:`Is Not Valid`
            (`self.SpawnTunnel` (`self.K2_GetActorLocation` (`GameplayStatics.GetPlayerPawn` 0)))))))))

(fn `SpawnTunnel`
  (params (SpawnLocation :type "Vector Structure"))
  (locals (NewLocalVar_0 :type "/Game/InfiniteMatrix/Blueprints/BP_Tunnel Object Reference"))
  (bind _spawnlocation (`self.SpawnLocation`))
  (bind _output_get (set `self.SpawnLocation` SpawnLocation))
  (bind _returnvalue (`|SpawnActorFromClass` "/Game/InfiniteMatrix/Blueprints/BP_Tunnel.BP_Tunnel_C" (`KismetMathLibrary.MakeTransform` _output_get) "Undefined" "OverrideRootScale" null null))
  (bind _output_get_2 (set `self.Newest Tunnel` _returnvalue))
  (set `/Game/InfiniteMatrix/Blueprints/BP_Tunnel.TunnelSpawner` self _output_get_2)
  (`|ExecutionSequence`
    (:`then_0`
      (`self.AddRandomHealthPack` _spawnlocation))
    (:`then_1`
      (`self.AddRandomEnemy` _spawnlocation))))

(fn `UserConstructionScript`)